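; TestNPC is a test NPC Blueprint that displays a chat box widget when it talks.
; Its Widget component is hidden on BeginPlay.
; DoTalk checks that NpcDataAsset is valid, unhides the widget and writes a hardcoded placeholder string to the NpcChatBox text.
; The data asset's contents are not read, and nothing here hides the box again after talking.
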(event `self.ReceiveBeginPlay`
  (`SceneComponent.SetHiddenInGame` (`self.Widget`) true false))

(event `/Game/Main/Blueprint/Instence/NpcInterface.DoTalk`
  (bind _widget (`self.Widget`))
  (if (`KismetSystemLibrary.IsValid` (`self.NpcDataAsset`))
    (`SceneComponent.SetHiddenInGame` _widget false false)
    (bind _asnpc_chat_box (cast `/Game/Main/UMG/Player/NpcChatBox` (`WidgetComponent.GetWidget` _widget)))
    (set `/Game/Main/UMG/Player/NpcChatBox.TextVar` "test" _asnpc_chat_box)))

(fn `UserConstructionScript`)