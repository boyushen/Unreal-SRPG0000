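; NPC character Blueprint whose modular appearance and dialogue come from an NpcDataAsset.
; On BeginPlay it hides the speech bubble, sets each body-part mesh from the asset and slaves the parts to the main Mesh via master pose.
; DoTalk shows the next line for the current SituationId in the NpcChatBox widget for two seconds.
; GetSpeechBubbleText restarts at the first line when the conversation index runs out.
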(event `self.ReceiveBeginPlay`
  (`SceneComponent.SetHiddenInGame` (`self.Speechbubble`) true false)
  (`self.SetMeshParts`
    (:`Out`
      (`SkinnedMeshComponent.SetLeaderPoseComponent` (`self.Belt`) (`self.Mesh`) false)
      (`SkinnedMeshComponent.SetLeaderPoseComponent` (`self.ShoulderPod`) (`self.Mesh`) false)
      (`SkinnedMeshComponent.SetLeaderPoseComponent` (`self.HeadGears`) (`self.Mesh`) false)
      (`SkinnedMeshComponent.SetLeaderPoseComponent` (`self.Shoe`) (`self.Mesh`) false)
      (`SkinnedMeshComponent.SetLeaderPoseComponent` (`self.Glove`) (`self.Mesh`) false)
      (`SkinnedMeshComponent.SetLeaderPoseComponent` (`self.Hair`) (`self.Mesh`) false)
      (`SkinnedMeshComponent.SetLeaderPoseComponent` (`self.Face`) (`self.Mesh`) false))))

(event `/Game/Main/Blueprint/Instence/NpcInterface.DoTalk`
  (if (`KismetSystemLibrary.IsValid` (`self.NpcDataAsset`))
    (bind _asnpc_chat_box (cast `/Game/Main/UMG/Player/NpcChatBox` (`WidgetComponent.GetWidget` (`self.Speechbubble`))))
    (bind _result (`self.GetSpeechBubbleText`))
    (set `self.ConverSationIndex` (+ (`self.ConverSationIndex`) 1))
    (set `/Game/Main/UMG/Player/NpcChatBox.TextVar` _result _asnpc_chat_box)
    (`SceneComponent.SetHiddenInGame` (`self.Speechbubble`) false false)
    (`KismetSystemLibrary.Delay` 2.0)
    (`SceneComponent.SetHiddenInGame` (`self.Speechbubble`) true false)))

(fn `GetSpeechBubbleText`
  (returns (result :type Text))
  (locals (speechData :type "NpcScriptDataTableRow Structure"))
  (bind (_sid _situationid _conversation) (break `NpcScriptDataTableRow` (`local.speechData`)))
  (for _array_element (`NpcDataAsset.scriptItems` (`self.NpcDataAsset`))
    (if (== (`.SituationId` (break `NpcScriptDataTableRow` _array_element)) (`self.SituationId`))
      (set `local.speechData` _array_element)
      (break)))
  (if (`KismetArrayLibrary.Array_IsValidIndex` _conversation (`self.ConverSationIndex`))
    (return (`KismetTextLibrary.Conv_StringToText` (`|GetArrayItem` _conversation (`self.ConverSationIndex`))))
    (else
      (set `self.ConverSationIndex` 0)
      (return (`KismetTextLibrary.Conv_StringToText` (`|GetArrayItem` _conversation))))))

(fn `UserConstructionScript`)