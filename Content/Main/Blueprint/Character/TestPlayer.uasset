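; Test player character Blueprint with camera-relative movement and a hook for talking to NPCs.
; The vertical and horizontal axes move it along the control rotation's yaw.
; On BeginPlay it binds a talk-click event that calls DoTalkMessage on NearNpc when valid.
; Sphere overlap events are empty; logic to set or clear NearNpc and toggle the PlayerTest UI is disconnected and never runs.
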(event `self.ReceiveBeginPlay`
  (add `self.OnClickTalk` (delegate `CustomEvent_0`)))

(event `CustomEvent_0`
  (if (`KismetSystemLibrary.IsValid` (`self.NearNpc`))
    (message `/Game/Main/Blueprint/Instence/NpcInterface.DoTalk` (`self.NearNpc`))))

(event `InputAxis|verticle`
  (params (AxisValue :type "Float (single-precision)"))
  (`self.AddMovementInput` (`KismetMathLibrary.GetForwardVector` (`KismetMathLibrary.MakeRotator` 0.0 0.0 (.yaw (`self.GetControlRotation`)))) AxisValue))

(event `InputAxis|horizontal`
  (params (AxisValue :type "Float (single-precision)"))
  (`self.AddMovementInput` (`KismetMathLibrary.GetRightVector` (`KismetMathLibrary.MakeRotator` 0.0 0.0 (.yaw (`self.GetControlRotation`)))) AxisValue))

(event `self.Sphere.OnComponentBeginOverlap`
  (params (OverlappedComponent :type "PrimitiveComponent Object Reference") (OtherActor :type "Actor Object Reference") (OtherComp :type "PrimitiveComponent Object Reference") (OtherBodyIndex :type Integer) (bFromSweep :type Boolean) (SweepResult :type "HitResult Structure (by ref)")))

(event `self.Sphere.OnComponentEndOverlap`
  (params (OverlappedComponent :type "PrimitiveComponent Object Reference") (OtherActor :type "Actor Object Reference") (OtherComp :type "PrimitiveComponent Object Reference") (OtherBodyIndex :type Integer)))

(fn `UserConstructionScript`)