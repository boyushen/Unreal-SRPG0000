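; UI manager Blueprint that opens and closes widgets by name.
; OpenUI re-adds a cached widget from the UIList map, or looks up its class in the WidgetContentsList data table, creates it, shows it and caches it.
; CloseUI removes the named widget from its parent, optionally dropping it from the map so the next open creates a fresh instance.
; Unknown names only print a not-found message.
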(fn `Close UI`
  (params (Name :type Name) (removeUI :type Boolean))
  (locals (UIName :type Name))
  (bind (_value _returnvalue) (`BlueprintMapLibrary.Map_Find` (`self.UIList`) (`local.UIName`)))
  (set `local.UIName` Name)
  (if _returnvalue
    (`Widget.RemoveFromParent` _value)
    (if removeUI
      (`BlueprintMapLibrary.Map_Remove` (`self.UIList`) (`local.UIName`)))
    (else
      (`KismetSystemLibrary.PrintString` "NotFind UI"))))

(fn `OpenUI`
  (params (uiName :type Name))
  (locals (Key :type Name))
  (bind (_value _returnvalue) (`BlueprintMapLibrary.Map_Find` (`self.UIList`) (`local.Key`)))
  (set `local.Key` uiName)
  (if _returnvalue
    (`UserWidget.AddToViewport` _value 0)
    (else
      (bind _returnvalue_2 (`|GetDataTableRow` "/Game/Main/Data/UI/Base/WidgetContentsList.WidgetContentsList" (`local.Key`))
        (:`then`
          (bind _returnvalue_3 (`|CreateWidget` (`.widget_8_970F724F49B961AAE8D69F8B8B063D53` (break `/Game/Main/Data/UI/Base/WidgetKeyLink` _returnvalue_2))))
          (`UserWidget.AddToViewport` _returnvalue_3 0)
          (`BlueprintMapLibrary.Map_Add` (`self.UIList`) (`local.Key`) _returnvalue_3))
        (:`RowNotFound`
          (`KismetSystemLibrary.PrintString` "NotFind"))))))